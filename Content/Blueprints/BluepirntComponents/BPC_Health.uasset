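; BPC_Health is a health component Blueprint that stores a current health value and changes it through two functions.
; AddHealth sums the amount and current health, then clamps the result between the minimum and maximum health.
; RemoveHealth clamps the same way but subtracts current health from the amount, the reverse of the order its name implies.
; The event graph holds no active logic.
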(fn `AddHealth`
  (params (Amount :type "Float (double-precision)"))
  (set `self.CurrentHealth` (`KismetMathLibrary.FClamp` (+ Amount (`self.CurrentHealth`)) (`self.MinHealth`) (`self.MaxHealth`))))

(fn `RemoveHealth`
  (params (Amount :type "Float (double-precision)"))
  (set `self.CurrentHealth` (`KismetMathLibrary.FClamp` (- Amount (`self.CurrentHealth`)) (`self.MinHealth`) (`self.MaxHealth`))))